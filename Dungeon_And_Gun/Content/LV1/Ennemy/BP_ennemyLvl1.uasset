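; Level 1 enemy Blueprint that chases the top-down player character when its PawnSensing component sees it.
; Each sighting sets CanSeeEnemy, starts an AI MoveTo toward the player and restarts a retriggerable TimeToForgot delay.
; When that delay expires without a new sighting, it clears the flag and wanders to a random reachable nearby point.
; Debug strings print on arrival; a forward line trace is left unwired.
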(event `self.PawnSensing.OnSeePawn`
  (params (Pawn :type "Pawn Object Reference"))
  ;[0.1146 0.1146 0.1146] Chasing player
  (bind _asbp_top_down_character (cast `/Game/TopDown/Blueprints/Characters/BP_TopDownCharacter` Pawn))
  (`|ExecutionSequence`
    (:`then_0`
      (set `self.canSeeEnemy` true)
      (`|AIMoveTo` self (0.0 0.0 0.0) _asbp_top_down_character
        (:`then`
          (`KismetSystemLibrary.PrintString` "See u" true true (struct :`R` 0.35694 :`B` 1.0 :`A` 1.0)))))
    (:`then_1`
      (`KismetSystemLibrary.RetriggerableDelay` (`self.timeToForgot`))
      (set `self.canSeeEnemy` false)
      (`|AIMoveTo` self (`NavigationSystemV1.K2_GetRandomReachablePointInRadius` (`self.K2_GetActorLocation`) 500.0 null null) null 5.0 true
        (:`then`
          (`KismetSystemLibrary.PrintString` "What was I chasing again ?" true true (struct :`R` 0.48295 :`B` 1.0 :`A` 1.0)))))))

(event `self.ReceiveBeginPlay`)

(fn `UserConstructionScript`)