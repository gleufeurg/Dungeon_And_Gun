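; Door actor that slides its mesh down to open and back up to close, driven by external OpenDoor and CloseDoor events.
; OpenDoor waits briefly, then fires a camera shake, a door-open effect scaled to the mesh's X scale and a positional sound.
; A timeline then lerps the mesh's relative location without sweeping.
; CloseDoor reverses that timeline with no effects of its own.
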(event `Open Door`
  (bind _returnvalue_x (`KismetMathLibrary.BreakVector` (`SceneComponent.K2_GetComponentScale` (`self.StaticMesh`))))
  (`KismetSystemLibrary.Delay` 0.2)
  (`MatineeCameraShake.StartMatineeCameraShake` (`GameplayStatics.GetPlayerCameraManager` 0) "/Game/TechArt/Door_box/ShakeDoor.ShakeDoor_C")
  (`NiagaraFunctionLibrary.SpawnSystemAtLocation` "/Game/TechArt/FX/Niagara/FX_DoorOpen.FX_DoorOpen" (`SceneComponent.K2_GetComponentLocation` (`self.Scene`)) (struct) (`KismetMathLibrary.MakeVector` _returnvalue_x 1.0 1.0))
  (`GameplayStatics.PlaySoundAtLocation` "/Game/SFX/MovingTextured1_Cue.MovingTextured1_Cue" (`SceneComponent.K2_GetComponentLocation` (`self.StaticMesh`)) (struct) 1.0 1.0 0.0 "/Game/SFX/Attenuations/NewSoundAttenuation.NewSoundAttenuation" null null null)
  (bind (_direction _open) (`Timeline|OpenDoor` :!label _label)
    (:`Update`
      (`SceneComponent.K2_SetRelativeLocation` (`self.StaticMesh`) (`KismetMathLibrary.VLerp` (0.0 0.0 0.0) (0.0 0.0 -300.0) _open) false false))))

(event `Close Door`
  (goto _label :!via `Reverse`))

(fn `UserConstructionScript`)