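; MoveableBoxBP is a box that becomes a physics object when the top-down player character touches it.
; An overlap on its Box component, filtered by a cast to BP_TopDownCharacter, turns on physics simulation for the Cube.
; A custom Destroy event respawns a new instance of the same class at SpawnTransform, then removes the old actor after a brief delay.
; The mass override on the Cube is unconnected.
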(event `self.Box.OnComponentBeginOverlap`
  (params (OverlappedComponent :type "PrimitiveComponent Object Reference") (OtherActor :type "Actor Object Reference") (OtherComp :type "PrimitiveComponent Object Reference") (OtherBodyIndex :type Integer) (bFromSweep :type Boolean) (SweepResult :type "HitResult Structure (by ref)"))
  (cast `/Game/TopDown/Blueprints/Characters/BP_TopDownCharacter` OtherActor)
  (`PrimitiveComponent.SetSimulatePhysics` (`self.Cube`) true))

(event `self.Destroy`
  (`|SpawnActorFromClass` (`GameplayStatics.GetObjectClass` self) (`self.Spawn Transform`) "Undefined" "OverrideRootScale" null null)
  (`KismetSystemLibrary.Delay` 0.002)
  (`self.K2_DestroyActor`))

(fn `UserConstructionScript`)