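; Pressure plate actor that opens every DoorBP whose DoorValue matches its PlateValue when an actor overlaps it, and closes them when the overlap ends.
; Each overlap event searches all DoorBP actors in the level, with no filter on the overlapping actor.
; Each match also triggers FX: a sound, a Niagara burst and a Pulse timeline driving the plate's emissive and a temporarily visible point light.
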(event `self.ReceiveActorBeginOverlap`
  (params (OtherActor :type "Actor Object Reference"))
  (bind _outactors (`GameplayStatics.GetAllActorsOfClass` "/Game/TechArt/Door_box/DoorBP.DoorBP_C"))
  (for _array_element _outactors
    (if (== (`/Game/TechArt/Door_box/DoorBP.DoorValue` _array_element) (`self.PlateValue`))
      (`self.FX`)
      (`/Game/TechArt/Door_box/DoorBP.Open Door` _array_element))))

(event `self.ReceiveActorEndOverlap`
  (params (OtherActor :type "Actor Object Reference"))
  (`GameplayStatics.GetAllActorsOfClass` "/Game/TechArt/Door_box/DoorBP.DoorBP_C")
  (for _array_element _
    (if (== (`/Game/A_Part/TechArt/Door_box/PressurPlateBP.DoorValue` _array_element) (`self.PlateValue`))
      (`self.FX`)
      (`self.Close Door` _array_element))))

(event `FX`
  (bind _pointlight (`self.PointLight`))
  (bind _returnvalue (`SceneComponent.K2_GetComponentLocation` (`self.Plane`)))
  (`SceneComponent.SetVisibility` (`self.PointLight`) true false)
  (`GameplayStatics.PlaySoundAtLocation` "/Game/SFX/Pad_SoftBright_Cue.Pad_SoftBright_Cue" _returnvalue (struct) 1.0 1.0 0.0 "/Game/SFX/Attenuations/NewSoundAttenuation.NewSoundAttenuation" null null null)
  (`NiagaraFunctionLibrary.SpawnSystemAtLocation` "/Game/TechArt/FX/Niagara/FX_Pressureplate.FX_Pressureplate" _returnvalue)
  (bind (_direction _pulse) (`Timeline|Pulse`)
    (:`Update`
      (`MeshComponent.SetVectorParameterValueOnMaterials` (`self.Plane`) "Emissive" (`KismetMathLibrary.Conv_LinearColorToVector` _pulse))
      (`LightComponent.SetLightColor` _pointlight _pulse true))
    (:`Finished`
      (`SceneComponent.SetVisibility` _pointlight false false))))

(fn `UserConstructionScript`)