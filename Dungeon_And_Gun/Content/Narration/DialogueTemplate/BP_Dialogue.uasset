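; Dialogue actor that plays scene lines from a data table in a UI_Dialogue widget, then opens level LV1Final and destroys itself.
; InitiateDialogue loads the rows and creates the widget, then PlayLine triggers each row's vignette animation and starts the text.
; A looping timer calls Typewriter to reveal one letter at a time with a talk sound.
; Space completes or advances a line, while Escape or Enter ends the dialogue.
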(event `InitiateDialogue`
  (params (CurrentDialogue :type "DataTable Object Reference") (typingSpeed :type "Float (double-precision)"))
  ;[1 1 1] Listage des lignes à afficher
  (set `self.typingSpeed` typingSpeed)
  (bind _outrownames (`DataTableFunctionLibrary.GetDataTableRowNames` CurrentDialogue)) ; On va chercher les lignes de la scene
  (for _array_element _outrownames
    (bind _returnvalue (`|GetDataTableRow` CurrentDialogue _array_element)
      (:`then`
        (`KismetArrayLibrary.Array_Add` (`self.rows 2`) _returnvalue))))
  (bind _returnvalue_2 (`|CreateWidget` "/Game/Narration/DialogueTemplate/UI_Dialogue.UI_Dialogue_C")) ; On affiche la boite de dialogue
  (bind _output_get (set `self.dialogueUI ref` _returnvalue_2))
  (`UserWidget.AddToViewport` _output_get 0)
  (`self.PlayLine`) ; On commence la 1ere ligne
)

(event `self.ReceiveBeginPlay`
  ;[1 1 1] Demare l'ecriture de la 1ere ligne
  (`self.EnableInput` (`GameplayStatics.GetPlayerController` 0))
  (`KismetSystemLibrary.K2_SetTimer` null "Typewriter" (`self.typingSpeed`) true) ; Ecriture des lignes selon la vitesse entre chaque lettres
)

(event `Key|SpaceBar`
  (params (Key :type "Key Structure"))
  (bind _output_text (break `/Game/Narration/DialogueTemplate/S_Scene` (`|GetArrayItem` (`self.rows 2`) (`self.row`))))
  (bind _textblock_0 (`/Game/Narration/DialogueTemplate/UI_Dialogue.TextBlock_0` (`self.dialogueUI ref`)))
  ;[1 1 1] Skip/Jouer la prochaine ligne
  (:`Pressed`
    (if (`self.rowFinished?`)
      (`/Engine/EditorBlueprintResources/StandardMacros.IncrementInt` (`self.row`) ; Passe prochaine ligne
        (:`  `
          (set `self.charactersToDisplay` 0) ; 0 lettres à afficher
          (`Widget.SetVisibility` _textblock_0 "Hidden")
          (`self.PlayLine`) ; On relance l'event mais à la prochaine ligne
        ))
      (else
        (set `self.charactersToDisplay` (`KismetStringLibrary.Len` _output_text))
        (set `self.rowFinished?` false)
        (`Widget.SetVisibility` _textblock_0 "Visible")))))

(event `PlayLine`
  (bind (_text _vignette _anim_) (break `/Game/Narration/DialogueTemplate/S_Scene` (`|GetArrayItem` (`self.rows 2`) (`self.row`))))
  ;[1 1 1] Ecriture Prochaine ligne
  (`/Game/Narration/DialogueTemplate/UI_Dialogue.Play Vignette Animation` (`self.dialogueUI ref`) _vignette _anim_)
  (set `self.rowFinished?` false)
  (if (>= (`self.row`) (`KismetArrayLibrary.Array_Length` (`self.rows 2`)))
    (`self.EndDialogue`)
    (else
      (`self.Typewriter`)
      (`KismetSystemLibrary.K2_SetTimer` null "Typewriter" (`self.typingSpeed`) true) ; On relance l'ecriture
    )))

(event `EndDialogue`
  ;[1 1 1] Fin Dialogue
  (`Widget.RemoveFromParent` (`self.dialogueUI ref`))
  (`GameplayStatics.OpenLevelBySoftObjectPtr` "/Game/A_Part/TechArt/LV1Final.LV1Final")
  (`self.K2_DestroyActor`) ; On detruit l'acteur du dialogue
)

(event `Key|Escape`
  (params (Key :type "Key Structure"))
  (:`Pressed`
    (`self.EndDialogue` :!label _label)))

(event `Key|Enter`
  (params (Key :type "Key Structure"))
  (:`Pressed`
    (goto _label)))

(fn `Typewriter`
  (bind _dialogueui_ref (`self.dialogueUI ref`))
  (bind _characterstodisplay (`self.charactersToDisplay`))
  (bind _output_text (break `/Game/Narration/DialogueTemplate/S_Scene` (`|GetArrayItem` (`self.rows 2`) (`self.row`))))
  (`/Engine/EditorBlueprintResources/StandardMacros.IncrementInt` _characterstodisplay ; Affiche une lettre en plus
    (:`  `
      (`/Engine/EditorBlueprintResources/StandardMacros.IsValid` _dialogueui_ref
        (:`Is Valid`
          (`RichTextBlock.SetText` (`/Game/Narration/DialogueTemplate/UI_Dialogue.TextBlock_Dialogue` _dialogueui_ref) (`KismetTextLibrary.Conv_StringToText` (`KismetStringLibrary.GetSubstring` _output_text 0 _characterstodisplay)))
          (if (< (`self.charactersToDisplay`) (`KismetStringLibrary.Len` (`.Text_5_C388421542242FC6FA0C2C9510A2F6EF` (break `/Game/Narration/DialogueTemplate/S_Scene` (`|GetArrayItem` (`self.rows 2`) (`self.row`))))))
            (`GameplayStatics.PlaySound2D` "/Game/Narration/DialogueTemplate/TalkSound_Cue.TalkSound_Cue" 1.0 1.0 0.0 null null) ; son d'ecriture du text
            (else
              (set `self.rowFinished?` true)
              (`Widget.SetVisibility` (`/Game/Narration/DialogueTemplate/UI_Dialogue.TextBlock_0` (`self.dialogueUI ref`)) "Visible") ; ligne terminée, en attente de skip pour prochaine ligne
            )))))))

(fn `UserConstructionScript`)