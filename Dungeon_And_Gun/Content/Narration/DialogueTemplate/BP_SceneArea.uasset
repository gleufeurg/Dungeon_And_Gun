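; BP_SceneArea is a trigger volume that starts a narration dialogue when the player pawn enters it.
; On box overlap it spawns a BP_Dialogue at its own transform, stores the reference and initiates it with its CurrentDialogue and a fixed typing speed.
; End overlap calls EndDialogue on the stored instance if valid, without checking which actor left.
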(event `self.Box.OnComponentBeginOverlap`
  (params (OverlappedComponent :type "PrimitiveComponent Object Reference") (OtherActor :type "Actor Object Reference") (OtherComp :type "PrimitiveComponent Object Reference") (OtherBodyIndex :type Integer) (bFromSweep :type Boolean) (SweepResult :type "HitResult Structure (by ref)"))
  (if (== OtherActor (`GameplayStatics.GetPlayerPawn` 0))
    (bind _returnvalue (`|SpawnActorFromClass` "/Game/Narration/DialogueTemplate/BP_Dialogue.BP_Dialogue_C" (`self.GetTransform`) "Undefined" "OverrideRootScale" null null))
    (set `self.Dialogue` _returnvalue)
    (`/Game/Narration/DialogueTemplate/BP_Dialogue.InitiateDialogue` _returnvalue (`self.Current Dialogue`) 0.06)))

(event `self.Box.OnComponentEndOverlap`
  (params (OverlappedComponent :type "PrimitiveComponent Object Reference") (OtherActor :type "Actor Object Reference") (OtherComp :type "PrimitiveComponent Object Reference") (OtherBodyIndex :type Integer))
  (bind _dialogue (`self.Dialogue`))
  (`/Engine/EditorBlueprintResources/StandardMacros.IsValid` _dialogue
    (:`Is Valid`
      (`/Game/Narration/DialogueTemplate/BP_Dialogue.EndDialogue` _dialogue))))

(fn `UserConstructionScript`)